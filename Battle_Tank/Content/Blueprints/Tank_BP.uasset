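; Player-controlled tank Blueprint that maps input to camera aiming, track driving and firing.
; On BeginPlay it passes its TankTurret and Barrel components to the turret and barrel reference setters.
; Aim axes yaw the AzimuthGimbal and pitch the SpringArm, scaled by delta time for frame-rate independence.
; Separate throttle axes drive the left and right tracks independently, and the Fire action calls Fire.
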(event `self.ReceiveBeginPlay`
  (`self.SetTurretReference` (`self.TankTurret`))
  (`self.SetBarrelReference` (`self.Barrel`)))

(event `InputAxis|AimAzimuth`
  (params (AxisValue :type "Float (single-precision)"))
  ;[1 1 1] Input Control oldalas
  (`SceneComponent.K2_AddLocalRotation` (`self.Azimuth Gimbal`) (`KismetMathLibrary.MakeRotator` 0.0 0.0 (* AxisValue (`GameplayStatics.GetWorldDeltaSeconds`) 100.0)) false false))

(event `InputAxis|Left Track Throttle`
  (params (AxisValue :type "Float (single-precision)"))
  ;[1 1 1] Set Throttle
  (`TankTrack.SetThrottle` (`self.LeftTrack`) AxisValue))

(event `InputAxis|Right Track Throttle`
  (params (AxisValue :type "Float (single-precision)"))
  ;[1 1 1] Set Throttle
  (`TankTrack.SetThrottle` (`self.RightTrack`) AxisValue))

(event `InputAxis|AimElevation`
  (params (AxisValue :type "Float (single-precision)"))
  ;[1 1 1] Input fel-le
  (`SceneComponent.K2_AddLocalRotation` (`self.SpringArm`) (`KismetMathLibrary.MakeRotator` 0.0 (* AxisValue (`GameplayStatics.GetWorldDeltaSeconds`) 100.0)) false false))

(event `InputAction|Fire`
  (params (Key :type "Key Structure"))
  ;[1 1 1] Fire input
  (:`Pressed`
    (`self.Fire`)))

(fn `UserConstructionScript`)